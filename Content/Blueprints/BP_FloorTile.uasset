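; Self-recycling floor tile that randomly populates itself with a blocker, coins or bombs.
; The construction script picks one kind, adding child actors at one of three spawn points for a blocker or randomly inside CoinArea for coins and a bomb.
; When BP_Player overlaps EndTrigger, the tile asks BP_GameMode to add another tile, then destroys itself after a short delay.
; GetAttacheTranform exposes the Attachepoint world transform.
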(event OnComponentBeginOverlap(EndTrigger)
  (params (OverlappedComponent :type Primitive%20Component%20Object%20Reference) (OtherActor :type Actor%20Object%20Reference) (OtherComp :type Primitive%20Component%20Object%20Reference) (OtherBodyIndex :type Integer) (bFromSweep :type Boolean) (SweepResult :type Hit%20Result%20Structure%20%28by%20ref%29))
  (Utilities|Casting|CastToBP_Player OtherActor)
  (bind _asbp_game_mode (Utilities|Casting|CastToBP_GameMode (Game|GetGameMode)))
  (Default|AddFloorTile _asbp_game_mode)
  (Utilities|FlowControl|Delay 2.0)
  (Actor|DestroyActor))

(fn ConstructionScript
  (CallFunction|SetSpawnPoints)
  (switch int (Math|Random|RandomIntegerinRange 0 2)
    (:Default
      (CallFunction|SpawnBlocker :!label _label))
    (:0
      (goto _label))
    (:1
      (CallFunction|SpawnCoins))
    (:2
      (CallFunction|SpawnBombs))))

(fn GetAttacheTranform
  (return (Transformation|GetWorldTransform (Variables|Default|GetAttachepoint))))

(fn SetSpawnPoints
  (Variables|Default|SetSpawnPoints (Utilities|Array|MakeArray (Transformation|GetRelativeTransform (Variables|Default|GetSpawnPointR)) (Transformation|GetRelativeTransform (Variables|Default|GetSpawnpointL)) (Transformation|GetRelativeTransform (Variables|Default|GetSpawnpoint)))))

(fn SpawnBlocker
  (bind _spawnpoints (Variables|Default|GetSpawnPoints))
  (AddComponent|AddChildActorComponent false (Utilities|Array|Get(acopy) _spawnpoints (Math|Random|RandomIntegerinRange 0 (Utilities|Array|LastIndex _spawnpoints)))))

(fn SpawnCoins
  (bind _coinarea (Variables|Default|GetCoinArea))
  (for _index (range 0 5)
    (AddComponent|AddChildActorComponent false (Math|Conversions|ToTransform(Vector) (Math|Random|RandomPointinBoundingBox (Variables|/Script/Engine.SceneComponent|GetRelativeLocation _coinarea) (Variables|/Script/Engine.BoxComponent|GetBoxExtent _coinarea))))))

(fn SpawnBombs
  (bind _coinarea (Variables|Default|GetCoinArea))
  (AddComponent|AddChildActorComponent false (Math|Conversions|ToTransform(Vector) (Math|Random|RandomPointinBoundingBox (Variables|/Script/Engine.SceneComponent|GetRelativeLocation _coinarea) (Variables|/Script/Engine.BoxComponent|GetBoxExtent _coinarea)))))